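; Enemy drone character with a random mesh that, when activated, chases the player and fires projectiles within range.
; Tick's random Delay paces shots, and each shot re-pins its level-dependent height.
; Hit flashes use a dynamic material; ramming the SpaceShip triggers death with shake, brief slow-motion, explosion and sound.
; In TutorialLevel, the initial enemy count identifies the phase, so the last enemy destroyed shows the next prompt or spawns BeastMode pickups.
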(event Custom|Flash
  (bind _enemymesh (Variables|Default|GetEnemyMesh))
  ;[1 1 1] Enemy Hit Body Flash
  (bind _returnvalue (Rendering|Material|CreateDynamicMaterialInstance _enemymesh 0 (Rendering|Material|GetMaterial _enemymesh 0) "None" :!class /Script/Engine.PrimitiveComponent))
  (Rendering|Material|SetScalarParameterValue _returnvalue "Bright" 1e+02 :!class /Script/Engine.MaterialInstanceDynamic)
  (Utilities|FlowControl|Delay 0.1)
  (Rendering|Material|SetScalarParameterValue _returnvalue "Bright" 1.0 :!class /Script/Engine.MaterialInstanceDynamic))

(event Custom|EnemyDeath
  (bind _returnvalue (Transformation|GetActorLocation))
  ;[1 1 1] Enemy Death
  (Class|LegacyCameraShake|StartLegacyCameraShake (Game|GetPlayerCameraManager 0) "/Game/Levels/Blueprint/Character/ExplosionShake.ExplosionShake_C" 1.0 "CameraLocal" "0, 0, 0")
  (Utilities|Time|SetGlobalTimeDilation 0.08)
  (Utilities|FlowControl|Delay 0.05)
  (Utilities|Time|SetGlobalTimeDilation 1.0)
  (Effects|SpawnEmitteratLocation "/Game/StarterContent/Particles/P_Explosion.P_Explosion" _returnvalue)
  (Audio|PlaySoundatLocation "/Game/StarterContent/Audio/Explosion01.Explosion01" _returnvalue "0, 0, 0" 1.0 1.0 0.0 0 0 0 0)
  (Actor|DestroyActor))

(event Custom|SetTutorialPhase
  ;[1 1 1] Set Tutorial Phase
  (bind _returnvalue (Game|GetCurrentLevelName true))
  (if (Utilities|Enum|Equal(Enum) _returnvalue "TutorialLevel")
    (bind _outactors (Actor|GetAllActorsOfClass "EnemyCharacter_C"))
    (Variables|Default|SetTutorialPahse (Utilities|Array|Length _outactors))))

(event Custom|LockZAxis
  (params (LocationZ :type Float%20%28double-precision%29))
  (bind _returnvalue (Transformation|GetActorTransform))
  ;[1 1 1] LockActorZAxis
  (Transformation|SetActorLocation (Math|Vector|MakeVector (.x (.location _returnvalue)) (.y (.location _returnvalue)) (Math|Float|Clamp(Float) (.z (.location _returnvalue)) LocationZ LocationZ)) false false))

(event Collision|EventHit
  (params (MyComp :type Primitive%20Component%20Object%20Reference) (Other :type Actor%20Object%20Reference) (OtherComp :type Primitive%20Component%20Object%20Reference) (bSelfMoved :type Boolean) (HitLocation :type Vector :default "0, 0, 0") (HitNormal :type Vector :default "0, 0, 0") (NormalImpulse :type Vector :default "0, 0, 0") (Hit :type Hit%20Result%20Structure%20%28by%20ref%29))
  ;[1 1 1] Death By Collision Enemy
  (Utilities|Casting|CastToSpaceShip Other)
  (CallFunction|EnemyDeath))

(event EventTick
  (params (DeltaSeconds :type Float%20%28single-precision%29))
  ;[1 1 1] Enemy AI
  (if (Variables|Default|GetActivate)
    (AI|Navigation|MovetoActor (AI|GetAIController self) (Game|GetPlayerCharacter 0) 4.5e+02 true true true 0)
    (Utilities|FlowControl|Delay (Math|Random|RandomFloatinRange 1.5 3.0))
    (if (<= (Transformation|GetDistanceTo (Game|GetPlayerCharacter 0)) 1.2e+03)
      (Game|SpawnActorfromClass "/Game/Levels/Blueprint/Actors/Projectile/ProjectTile.ProjectTile_C" (Transformation|GetWorldTransform (Variables|Default|GetEnemy%20Projectile%20Transform)) "AlwaysSpawn" "MultiplyWithRoot" 0 self 0)
      (CallFunction|LockZAxis (Variables|Default|GetZAxis)))))

(event EventBeginPlay
  ;[1 1 1] Begin Play
  (bind _returnvalue (Game|GetCurrentLevelName true))
  (if (Utilities|Enum|Equal(Enum) _returnvalue "TutorialLevel")
    ;;[1 1 1] Delay to let the game spawn all enemies
    (Utilities|FlowControl|Delay 0.1)
    (CallFunction|SetTutorialPhase)
    (Variables|Default|SetZAxis 125.0)
    (else
      (Variables|Default|SetZAxis 265.0))))

(event EventDestroyed
  ;[1 1 1] On Destroyed
  (if (not (== 0 (Variables|Default|GetTutorialPahse)))
    (switch int (Variables|Default|GetTutorialPahse)
      (:2
        (bind _outactors (Actor|GetAllActorsOfClass "EnemyCharacter_C"))
        (if (== (Utilities|Array|Length _outactors) 1)
          (bind _foundwidgets (Widget|GetAllWidgetsOfClass "/Game/Levels/TutorialLevel/Widgets/DestroyEnemiesWidget.DestroyEnemiesWidget_C" true))
          (if (== (Utilities|Array|Length _foundwidgets) 1)
            (Widget|RemovefromParent (Utilities|Array|Get(acopy) _foundwidgets)))
          (bind _returnvalue (UserInterface|CreateWidget "/Game/Levels/TutorialLevel/Widgets/AfterEnemyPhaseOneWidget.AfterEnemyPhaseOneWidget_C"))
          (UserInterface|Viewport|AddtoViewport _returnvalue 0)))
      (:3
        (bind _outactors_2 (Actor|GetAllActorsOfClass "EnemyCharacter_C"))
        (if (== (Utilities|Array|Length _outactors_2) 1)
          (bind _returnvalue_2 (UserInterface|CreateWidget "/Game/Levels/TutorialLevel/Widgets/TakeHealthPickupsWidget.TakeHealthPickupsWidget_C"))
          (UserInterface|Viewport|AddtoViewport _returnvalue_2 0)))
      (:4
        (bind _outactors_3 (Actor|GetAllActorsOfClass "EnemyCharacter_C"))
        (if (== (Utilities|Array|Length _outactors_3) 1)
          (bind _returnvalue_3 (UserInterface|CreateWidget "/Game/Levels/TutorialLevel/Widgets/TakeBeastModeWidget.TakeBeastModeWidget_C"))
          (UserInterface|Viewport|AddtoViewport _returnvalue_3 0)
          (Game|SpawnActorfromClass "/Game/Levels/Blueprint/Actors/BeastMode/BeastMode.BeastMode_C" (Math|Transform|MakeTransform "19810.000000,3020.000000,100.000000" "0, 0, 0" "1.000000,1.000000,1.000000") "Undefined" "MultiplyWithRoot" 0 0)
          (Game|SpawnActorfromClass "/Game/Levels/Blueprint/Actors/BeastMode/BeastMode.BeastMode_C" (Math|Transform|MakeTransform "20040.000000,3020.000000,100.000000" "0, 0, 0" "1.000000,1.000000,1.000000") "Undefined" "MultiplyWithRoot" 0 0)))
      (:5
        (bind _outactors_4 (Actor|GetAllActorsOfClass "EnemyCharacter_C"))
        (if (== (Utilities|Array|Length _outactors_4) 1)
          (bind _returnvalue_4 (UserInterface|CreateWidget "/Game/Levels/TutorialLevel/Widgets/TakeCoinWidget.TakeCoinWidget_C"))
          (UserInterface|Viewport|AddtoViewport _returnvalue_4 0))))))

(fn ConstructionScript
  (Components|StaticMesh|SetStaticMesh (Variables|Default|GetEnemyMesh) (Utilities|Select :Index (Math|Random|RandomIntegerinRange 0 7) :Option%200 "/Game/Levels/Blueprint/Character/Mesh/Drone_V1_SciFi_FBX.Drone_V1_SciFi_FBX" :Option%201 "/Game/Levels/Blueprint/Character/Mesh/Drone_V2_SciFi_FBX.Drone_V2_SciFi_FBX" :Option%202 "/Game/Levels/Blueprint/Character/Mesh/Drone_V3_SciFi_FBX.Drone_V3_SciFi_FBX" :Option%203 "/Game/Levels/Blueprint/Character/Mesh/Drone_V4_SciFi_FBX.Drone_V4_SciFi_FBX" :Option%204 "/Game/Levels/Blueprint/Character/Mesh/Drone_V5_SciFi_FBX.Drone_V5_SciFi_FBX" :Option%205 "/Game/Levels/Blueprint/Character/Mesh/Drone_V6_SciFi_FBX.Drone_V6_SciFi_FBX" :Option%206 "/Game/Levels/Blueprint/Character/Mesh/Drone_V7_SciFi_FBX.Drone_V7_SciFi_FBX" :Option%207 "/Game/Levels/Blueprint/Character/Mesh/Drone_V8_SciFi_FBX.Drone_V8_SciFi_FBX")))