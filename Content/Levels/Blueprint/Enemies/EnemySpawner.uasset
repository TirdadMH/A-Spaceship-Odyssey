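; Level spawner actor that creates and later wakes EnemyCharacter AI when the player's SpaceShip enters its trigger volumes.
; Overlapping the SpawnEnemy volume spawns an AI enemy with a default controller at each SpawnTransform entry and stores it in EnemiesArray.
; Overlapping the ActivateEnemy volume sets Activate on every valid stored enemy.
; Each trigger responds only once through DoOnce, so spawning and activation are staged separately.
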(event OnComponentBeginOverlap(SpawnEnemy)
  (params (OverlappedComponent :type Primitive%20Component%20Object%20Reference) (OtherActor :type Actor%20Object%20Reference) (OtherComp :type Primitive%20Component%20Object%20Reference) (OtherBodyIndex :type Integer) (bFromSweep :type Boolean) (SweepResult :type Hit%20Result%20Structure%20%28by%20ref%29))
  ;[1 1 1] Enemy Spawner Logic
  (Utilities|Casting|CastToSpaceShip OtherActor)
  (Utilities|FlowControl|DoOnce false
    (:Completed
      (for _array_element (Variables|Default|GetSpawnTransform)
        (bind _returnvalue (AI|SpawnAIFromClass "/Game/Levels/Blueprint/Enemies/EnemyCharacter.EnemyCharacter_C" 0 (.Location (Math|Transform|BreakTransform _array_element)) (.Rotation (Math|Transform|BreakTransform _array_element)) true 0))
        (Pawn|SpawnDefaultController _returnvalue)
        (bind _asenemy_character (Utilities|Casting|CastToEnemyCharacter _returnvalue))
        (Utilities|Array|Add (Variables|Default|GetEnemiesArray) _asenemy_character)))))

(event OnComponentBeginOverlap(ActivateEnemy)
  (params (OverlappedComponent :type Primitive%20Component%20Object%20Reference) (OtherActor :type Actor%20Object%20Reference) (OtherComp :type Primitive%20Component%20Object%20Reference) (OtherBodyIndex :type Integer) (bFromSweep :type Boolean) (SweepResult :type Hit%20Result%20Structure%20%28by%20ref%29))
  ;[1 1 1] Enemy Activate Logic
  (Utilities|Casting|CastToSpaceShip OtherActor)
  (Utilities|FlowControl|DoOnce false
    (:Completed
      (for _array_element (Variables|Default|GetEnemiesArray)
        (Utilities|IsValid _array_element
          (:Is%20Valid
            (Variables|/Game/Levels/Blueprint/Enemies/EnemyCharacter.EnemyCharacter_C|SetActivate _array_element true)))))))

(fn ConstructionScript)